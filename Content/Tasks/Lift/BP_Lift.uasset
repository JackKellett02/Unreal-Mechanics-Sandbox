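; BP_Lift is a lift actor that moves between two positions when a CPP_Character overlaps its Trigger.
; BeginPlay stores the start location and treats EndPos as an offset from it.
; LiftTimeline plays or reverses according to GoToStartPos, lerping the location without sweep along LiftCurve.
; A FlipFlop on timeline completion toggles the direction for the next overlap; the InvertGoToStartPos helper is not called here.
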(event `self.ReceiveBeginPlay`
  (set `self.StartPos` (`self.K2_GetActorLocation`))
  (set `self.EndPos` (+ (`self.K2_GetActorLocation`) (`self.EndPos`))))

(event `self.Trigger.OnComponentBeginOverlap`
  (params (OverlappedComponent :type "PrimitiveComponent Object Reference") (OtherActor :type "Actor Object Reference") (OtherComp :type "PrimitiveComponent Object Reference") (OtherBodyIndex :type Integer) (bFromSweep :type Boolean) (SweepResult :type "HitResult Structure (by ref)"))
  (cast `CPP_Character` OtherActor)
  (if (`self.GoToStartPos`)
    (bind (_direction _liftcurve) (`Timeline|LiftTimeline` :!via `Reverse` :!label _label)
      (:`Update`
        (`self.K2_SetActorRelativeLocation` (`KismetMathLibrary.VLerp` (`self.StartPos`) (`self.EndPos`) _liftcurve)))
      (:`Finished`
        (`/Engine/EditorBlueprintResources/StandardMacros.FlipFlop`
          (:`A`
            (set `self.GoToStartPos` true))
          (:`B`
            (set `self.GoToStartPos` false)))))
    (else
      (goto _label))))

(fn `InvertGoToStartPos`
  (returns (`starpos?` :type Boolean))
  (if (`self.GoToStartPos`)
    (set `self.GoToStartPos` false)
    (else
      (set `self.GoToStartPos` true)))
  (return (`self.GoToStartPos`)))

(fn `UserConstructionScript`)