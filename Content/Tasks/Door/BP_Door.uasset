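; BP_Door is a door actor that rotates open while something overlaps it and swings back when the overlap ends.
; BeginPlay caches the starting rotation, and overlap events from any actor toggle the ShouldDoorOpen flag.
; Tick lerps the current rotation toward DesiredRotation or the cached start by a fixed alpha, giving an eased, frame-rate-dependent swing.
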(event `self.ReceiveBeginPlay`
  (set `self.startingRotation` (`self.K2_GetActorRotation`)))

(event `self.ReceiveActorBeginOverlap`
  (params (OtherActor :type "Actor Object Reference"))
  (set `self.ShouldDoorOpen` true))

(event `self.ReceiveActorEndOverlap`
  (params (OtherActor :type "Actor Object Reference"))
  (set `self.ShouldDoorOpen` false))

(event `self.ReceiveTick`
  (params (DeltaSeconds :type "Float (single-precision)"))
  (if (`self.ShouldDoorOpen`)
    (`self.K2_SetActorRotation` (`KismetMathLibrary.RLerp` (`self.K2_GetActorRotation`) (`self.DesiredRotation`) 0.1))
    (else
      (`self.K2_SetActorRotation` (`KismetMathLibrary.RLerp` (`self.K2_GetActorRotation`) (`self.startingRotation`) 0.1)))))

(fn `UserConstructionScript`)